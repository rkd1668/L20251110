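; BP_Rocket is a rocket projectile that explodes when it overlaps an actor tagged "Target".
; On that overlap it applies damage credited to the first player controller and spawns an explosion sound and particle effect at its location.
; It then calls GameCheck on the BP_GM game mode and destroys itself, which only happens if that cast succeeds.
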(event `self.ReceiveAnyDamage`
  (params (Damage :type "Float (single-precision)") (DamageType :type "DamageType Object Reference") (InstigatedBy :type "Controller Object Reference") (DamageCauser :type "Actor Object Reference")))

(event `self.ReceiveBeginPlay`)

(event `self.ReceiveActorBeginOverlap`
  (params (OtherActor :type "Actor Object Reference"))
  (if (`self.ActorHasTag` OtherActor "Target")
    (`GameplayStatics.ApplyDamage` OtherActor 100.0 (`GameplayStatics.GetPlayerController` 0) self)
    (`GameplayStatics.SpawnSoundAtLocation` "/Game/StarterContent/Audio/Explosion_Cue.Explosion_Cue" (`self.K2_GetActorLocation`) (struct) 1.0 1.0 0.0 null null)
    (`GameplayStatics.SpawnEmitterAtLocation` "/Game/StarterContent/Particles/P_Explosion.P_Explosion" (`self.K2_GetActorLocation`))
    (bind _asbp_gm (cast `/Game/Blueprints/BP_GM` (`GameplayStatics.GetGameMode`)))
    (`/Game/Blueprints/BP_GM.GameCheck` _asbp_gm)
    (`self.K2_DestroyActor`)))

(fn `UserConstructionScript`)