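; BP_P38 is a player-flown plane pawn that constantly moves forward and fires rockets.
; Tick feeds movement input along the actor's forward vector every frame.
; The IA_Movement Enhanced Input action applies frame-rate-scaled local rotations, pitching on Y and rolling on X, with no yaw control.
; IA_Fire spawns a BP_Rocket at the Arrow component's transform, with the plane as owner and instigator.
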(event `self.ReceiveTick`
  (params (DeltaSeconds :type "Float (single-precision)"))
  (`self.AddMovementInput` (`self.GetActorForwardVector`)))

(event `EnhancedInput|/Game/Blueprints/Input/IA_Movement`
  (params (ActionValue :type "Vector2D Structure") (ElapsedSeconds :type "Float (double-precision)") (TriggeredSeconds :type "Float (double-precision)") (InputAction :type "InputAction Object Reference" :default "/Game/Blueprints/Input/IA_Movement.IA_Movement"))
  (:`Triggered`
    (`self.K2_AddActorLocalRotation` (`KismetMathLibrary.MakeRotator` 0.0 (* ActionValue_Y (`GameplayStatics.GetWorldDeltaSeconds`) 60.0)))
    (`self.K2_AddActorLocalRotation` (`KismetMathLibrary.MakeRotator` (* ActionValue_X (`GameplayStatics.GetWorldDeltaSeconds`) 60.0)))))

(event `InputAction|Fire`
  (params (Key :type "Key Structure")))

(event `EnhancedInput|/Game/Blueprints/Input/IA_Fire`
  (params (ActionValue :type Boolean) (ElapsedSeconds :type "Float (double-precision)") (TriggeredSeconds :type "Float (double-precision)") (InputAction :type "InputAction Object Reference" :default "/Game/Blueprints/Input/IA_Fire.IA_Fire"))
  (:`Triggered`
    (`|SpawnActorFromClass` "/Game/Blueprints/BP_Rocket.BP_Rocket_C" (`SceneComponent.K2_GetComponentToWorld` (`self.Arrow`)) "Undefined" "MultiplyWithRoot" self self)))

(fn `UserConstructionScript`)