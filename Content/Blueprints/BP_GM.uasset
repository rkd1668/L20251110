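; BP_GM handles stage clearing, advancing to the next level once no actors tagged "Target" remain.
; The GameCheck event counts tagged actors and, at zero, prints a Korean next-stage message, then calls OpenLevelByName(Test) after a short delay.
; That function derives the next Step0N level from the current name's digit using ASCII arithmetic, wrapping from Step03 back to Step01.
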(event `GameCheck`
  (bind _outactors (`GameplayStatics.GetAllActorsWithTag` "Target"))
  (if (== (`KismetArrayLibrary.Array_Length` _outactors) 0)
    (`KismetSystemLibrary.PrintString` "다음 스테이지로")
    (`KismetSystemLibrary.Delay` 3.0)
    (`self.OpenLevelByName(Test)`)))

(fn `OpenLevelByName(Test)`
  (bind _stepnumber (`self.StepNumber`))
  (bind _returnvalue (`GameplayStatics.GetCurrentLevelName` true))
  (bind _output_get (set `self.StepNumber` (+ (`KismetStringLibrary.GetCharacterAsNumber` (`KismetStringLibrary.GetSubstring` _returnvalue 5)) 1)))
  (if (> _output_get 51)
    (set `self.StepNumber` 1)
    (else
      (set `self.StepNumber` (- _stepnumber 48))))
  (`GameplayStatics.OpenLevel` (`KismetStringLibrary.Conv_StringToName` (`KismetStringLibrary.Concat_StrStr` "Step0" (`KismetStringLibrary.Conv_IntToString` _stepnumber)))))

(fn `UserConstructionScript`)